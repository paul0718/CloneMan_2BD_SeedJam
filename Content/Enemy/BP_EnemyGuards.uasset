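; Enemy guard Blueprint with a laser beam that shortens against obstacles and collision that turns off on death.
; Each tick, LaserTick traces the Visibility channel along the laser's forward vector, flattened to horizontal, up to a maximum distance.
; It writes the 2D hit distance, or the maximum on a miss, into the effect's "Beam End" parameter.
; BeginPlay binds the health component's death event to disable actor collision.
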(event Custom|Disable%20Collision
  (Collision|SetActorEnableCollision false))

(event EventBeginPlay
  (EventDispatchers|BindEventtoOnDeath (Variables|Default|GetAC_HealthComp) (delegate Custom|Disable%20Collision)))

(event Collision|EventActorBeginOverlap
  (params (OtherActor :type Actor%20Object%20Reference)))

(event EventTick
  (params (DeltaSeconds :type Float%20%28single-precision%29))
  (CallFunction|LaserTick (Variables|Default|GetNS_Laser) (Variables|Default|GetLaserMaxDist)))

(fn ConstructionScript)

(fn LaserTick
  (params (TargetLaserRef :type Niagara%20Component%20Object%20Reference%20%28by%20ref%29) (MaxDistance :type Float%20%28double-precision%29))
  (bind _returnvalue (Transformation|GetWorldLocation TargetLaserRef))
  (bind _returnvalue_2 (Math|Vector|GetForwardVector TargetLaserRef))
  (bind (_outhit _returnvalue_3) (Collision|LineTraceByChannel _returnvalue (+ _returnvalue (* (Math|Vector|MakeVector (.x _returnvalue_2) (.y _returnvalue_2) 0.0) MaxDistance)) "TraceTypeQuery1" true 0 "None" true "(R=1.000000,G=0.000000,B=0.844550,A=1.000000)" "(R=1.000000,G=0.538341,B=0.000000,A=1.000000)" 0.1))
  (if _returnvalue_3
    (Effects|Components|ParticleSystem|SetVectorParameter TargetLaserRef "Beam End" (Math|Vector|MakeVector (Math|Vector|Distance2D(Vector) (.Location (Collision|BreakHitResult _outhit)) (Transformation|GetWorldLocation TargetLaserRef)) 0.0 0.0))
    (else
      (Effects|Components|ParticleSystem|SetVectorParameter TargetLaserRef "Beam End" (Math|Vector|MakeVector MaxDistance 0.0 0.0)))))