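; BP_Door_Automatic is a laboratory sliding door that opens and closes automatically through a trigger box.
; Box begin overlap plays Timeline_Door and end overlap reverses it, with no filter on the overlapping actor.
; The timeline curve slides the two door leaves apart along local Y in opposite directions.
; Each overlap event also plays a 3D sound at the door frame through an audio manager call using the GameState.
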(event OnComponentBeginOverlap(Box)
  (params (OverlappedComponent :type Primitive%20Component%20Object%20Reference) (OtherActor :type Actor%20Object%20Reference) (OtherComp :type Primitive%20Component%20Object%20Reference) (OtherBodyIndex :type Integer) (bFromSweep :type Boolean) (SweepResult :type Hit%20Result%20Structure%20%28by%20ref%29))
  (CallFunction|AudioManagerPlaySound (Game|GetGameState) "NewEnumerator18" true (Transformation|GetWorldLocation (Variables|Default|GetDoor_Frame)))
  (bind _door_b (Timeline|Timeline_Door Play)
    (:Update
      (Transformation|SetRelativeLocation (Variables|Default|GetDoor_A1) (Math|Vector|MakeVector 0.0 (* _door_b 85.0) 0.0) false false)
      (Transformation|SetRelativeLocation (Variables|Default|GetDoor_A2) (Math|Vector|MakeVector 0.0 (* _door_b -85.0) 0.0) false false))))

(event OnComponentEndOverlap(Box)
  (params (OverlappedComponent :type Primitive%20Component%20Object%20Reference) (OtherActor :type Actor%20Object%20Reference) (OtherComp :type Primitive%20Component%20Object%20Reference) (OtherBodyIndex :type Integer))
  (CallFunction|AudioManagerPlaySound (Game|GetGameState) "NewEnumerator27" true (Transformation|GetSocketLocation (Variables|Default|GetDoor_Frame) "None"))
  (bind _door_b (Timeline|Timeline_Door Reverse)
    (:Update
      (Transformation|SetRelativeLocation (Variables|Default|GetDoor_A1) (Math|Vector|MakeVector 0.0 (* _door_b 85.0) 0.0) false false)
      (Transformation|SetRelativeLocation (Variables|Default|GetDoor_A2) (Math|Vector|MakeVector 0.0 (* _door_b -85.0) 0.0) false false))))

(event EventBeginPlay)

(event Collision|EventActorBeginOverlap
  (params (OtherActor :type Actor%20Object%20Reference)))

(event EventTick
  (params (DeltaSeconds :type Float%20%28single-precision%29)))

(fn ConstructionScript)