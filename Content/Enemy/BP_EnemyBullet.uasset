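; BP_EnemyBullet is an enemy projectile that deals fixed damage on overlap and destroys itself after a short lifetime.
; Its sphere overlap casts the other actor and calls TakeDamageEvent on the health component of a BP_DeathBlocker or the top-down player.
; The bullet is destroyed on hitting a blocker or any unrelated actor, but not on hitting the player or enemy guards.
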(event OnComponentHit(Sphere)
  (params (HitComponent :type Primitive%20Component%20Object%20Reference) (OtherActor :type Actor%20Object%20Reference) (OtherComp :type Primitive%20Component%20Object%20Reference) (NormalImpulse :type Vector :default "0, 0, 0") (Hit :type Hit%20Result%20Structure%20%28by%20ref%29)))

(event OnComponentBeginOverlap(Sphere)
  (params (OverlappedComponent :type Primitive%20Component%20Object%20Reference) (OtherActor :type Actor%20Object%20Reference) (OtherComp :type Primitive%20Component%20Object%20Reference) (OtherBodyIndex :type Integer) (bFromSweep :type Boolean) (SweepResult :type Hit%20Result%20Structure%20%28by%20ref%29))
  (bind _output_get (Variables|Default|SetHitActor OtherActor))
  (bind _asbp_death_blocker (Utilities|Casting|CastToBP_DeathBlocker _output_get)
    (:then
      (Default|TakeDamageEvent (Variables|/Game/Animation/BP_DeathBlocker.BP_DeathBlocker_C|GetAC_HealthComp _asbp_death_blocker) 2e+01 self)
      (Actor|DestroyActor))
    (:CastFailed
      (bind _asbp_top_down_character (Utilities|Casting|CastToBP_TopDownCharacter (Variables|Default|GetHitActor))
        (:then
          (Default|TakeDamageEvent (Variables|/Game/TopDown/Blueprints/BP_TopDownCharacter.BP_TopDownCharacter_C|GetAC_HealthComp _asbp_top_down_character) 2e+01 self)
          (Development|PrintString "SHOT PLAYER"))
        (:CastFailed
          (Utilities|Casting|CastToBP_EnemyGuards (Variables|Default|GetHitActor)
            (:CastFailed
              (Actor|DestroyActor))))))))

(event EventBeginPlay
  (Utilities|FlowControl|Delay 2.0)
  (Actor|DestroyActor))

(event EventTick
  (params (DeltaSeconds :type Float%20%28single-precision%29)))

(fn ConstructionScript)