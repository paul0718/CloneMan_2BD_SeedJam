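; B_Cable is a construction-time spline actor that lays cable meshes along an editable spline.
; The construction script divides the spline length by a target Length, rounds to a segment count, and stretches each segment evenly to fit.
; Each added spline mesh component takes positions and length-clamped tangents from the spline, plus a uniform cross-section Scale and a decal-receiving toggle.
; The event graph has no runtime logic.
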(event EventBeginPlay)

(event Collision|EventActorBeginOverlap
  (params (OtherActor :type Actor%20Object%20Reference)))

(event EventTick
  (params (DeltaSeconds :type Float%20%28single-precision%29)))

(fn ConstructionScript
  (bind _spline (Variables|Default|GetSpline))
  (bind _length (Variables|Default|GetLength))
  (bind _spline_2 (Variables|Default|GetSpline))
  (bind _length_2 (Variables|Default|GetLength))
  (bind _scale (Variables|General|GetScale))
  (bind _returnvalue (Spline|GetSplineLength _spline_2))
  (bind _returnvalue_2 (Math|Vector2D|MakeVector2D _scale _scale))
  (bind _returnvalue_3 (/ _returnvalue _length))
  (bind _returnvalue_4 (Math|Float|Round _returnvalue_3))
  (Variables|Default|SetCurrentDistance 0.0)
  (Variables|Default|SetRealLeangth (/ _returnvalue (Math|Conversions|ToFloat(Integer) _returnvalue_4)))
  (bind _output_get (Variables|Default|SetNumberOfSegments _returnvalue_4))
  (for _index (range 0 (- _output_get 1))
    (bind _returnvalue_5 (AddComponent|AddSplineMeshComponent false))
    (SplineMesh|SetStartandEnd _returnvalue_5 (Spline|GetLocationatDistanceAlongSpline _spline (Variables|Default|GetCurrentDistance) "Local") (Math|Vector|ClampVectorSize (Spline|GetTangentatDistanceAlongSpline _spline (Variables|Default|GetCurrentDistance) "Local") 0.0 _length_2) (Spline|GetLocationatDistanceAlongSpline _spline (+ (Variables|Default|GetCurrentDistance) (Variables|Default|GetRealLeangth)) "Local") (Math|Vector|ClampVectorSize (Spline|GetTangentatDistanceAlongSpline _spline (+ (Variables|Default|GetCurrentDistance) (Variables|Default|GetRealLeangth)) "Local") 0.0 _length_2) true :!class /Script/Engine.SplineMeshComponent)
    (SplineMesh|SetStartScale _returnvalue_5 _returnvalue_2 true :!class /Script/Engine.SplineMeshComponent)
    (SplineMesh|SetEndScale _returnvalue_5 _returnvalue_2 true :!class /Script/Engine.SplineMeshComponent)
    (Variables|Default|SetCurrentDistance (+ (Variables|Default|GetCurrentDistance) (Variables|Default|GetRealLeangth)))
    (Rendering|SetReceivesDecals _returnvalue_5 (Variables|General|GetRecieve%20Decals))))