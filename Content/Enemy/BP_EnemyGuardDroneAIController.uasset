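; AI controller for the guard drone enemy that defines what happens when the drone dies.
; Its death effect stops the brain logic, deactivates the laser, unpossesses the pawn, makes the capsule ignore pawn and world-dynamic collision, and plays a one-shot death animation, replacing the parent's version.
; The death sound plays through the audio manager as 3D audio at the drone's location.
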(event EventBeginPlay
  (|CallParentFunction) ; This node is disabled and will not be called.\nDrag off pins to build functionality.
)

(event EventTick
  (params (DeltaSeconds :type Float%20%28single-precision%29))
  (|CallParentFunction DeltaSeconds) ; This node is disabled and will not be called.\nDrag off pins to build functionality.
)

(fn ConstructionScript
  (|CallParentFunction))

(fn EnemyDeathEffect
  (bind _enemyactor (Variables|Default|GetEnemyActor))
  (bind _enemyactor_2 (Variables|Default|GetEnemyActor))
  (bind _capsulecomponent (Variables|/Script/Engine.Character|GetCapsuleComponent _enemyactor))
  (bind _mesh (Variables|/Script/Engine.Character|GetMesh _enemyactor_2))
  (AI|Logic|StopLogic (Variables|Default|GetBrainComponent) "")
  (Components|Activation|Deactivate (Variables|Default|GetEnemyLaser))
  (Pawn|UnPossess)
  (Collision|SetCollisionResponsetoChannel _capsulecomponent "ECC_Pawn" "ECR_Ignore")
  (Collision|SetCollisionResponsetoChannel _capsulecomponent "ECC_WorldDynamic" "ECR_Ignore")
  (Components|Animation|SetAnimationMode _mesh "AnimationSingleNode" true)
  (Components|Animation|PlayAnimation _mesh "/Game/MilitaryDrone/Animations/anim_drone_death.anim_drone_death" false))

(fn EnemyDeathSound
  (CallFunction|AudioManagerPlaySound (Game|GetGameState) "NewEnumerator28" true (Transformation|GetActorLocation (Variables|Default|GetEnemyActor))))