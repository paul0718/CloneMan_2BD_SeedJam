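; Parent Blueprint for a switch indicator light that can be turned on, turned off or toggled through events.
; The construction script applies the mesh, a steady or blinking material, dirt and blink rate, then sets the initial light state.
; All state changes feed SetLight, which drives emissive and color material parameters.
; An optional off color keeps the light emissive and swaps color instead of going dark.
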(event Custom|Turn%20ON
  (Variables|Default|SetON true)
  (CallFunction|SetLight))

(event Custom|Turn%20OFF
  (Variables|Default|SetON false)
  (CallFunction|SetLight))

(event Custom|Toggle%20ON/OFF
  (Variables|Default|SetON (not (Variables|Default|GetON)))
  (CallFunction|SetLight))

(event EventBeginPlay)

(event Collision|EventActorBeginOverlap
  (params (OtherActor :type Actor%20Object%20Reference)))

(event EventTick
  (params (DeltaSeconds :type Float%20%28single-precision%29)))

(fn ConstructionScript
  (Utilities|FlowControl|Sequence
    (:then_0
      (Components|StaticMesh|SetStaticMesh (Variables|Default|GetSM_Indicator) (Variables|Default|GetMesh)))
    (:then_1
      (Rendering|Material|SetMaterial (Variables|Default|GetSM_Indicator) 0 (select (Variables|Default|GetBlinking) "/Game/BeautifulCorner/Switches/Buttons_and_Levers/Materials/Buttons_Indicators/MI_Buttons_Indicators_Blinking.MI_Buttons_Indicators_Blinking" "/Game/BeautifulCorner/Switches/Buttons_and_Levers/Materials/Buttons_Indicators/MI_Buttons_Indicators.MI_Buttons_Indicators")))
    (:then_2
      (Rendering|Material|SetScalarParameterValueonMaterials (Variables|Default|GetSM_Indicator) "Dirty" (Variables|Default|GetDirty)))
    (:then_3
      (CallFunction|SetLight)
      (Rendering|Material|SetScalarParameterValueonMaterials (Variables|Default|GetSM_Indicator) "Blinking Rate" (Variables|Default|GetBlinking%20Rate)))))

(fn SetLight
  (bind _indicator_color (Variables|Default|GetIndicator%20Color))
  (Rendering|Material|SetScalarParameterValueonMaterials (Variables|Default|GetSM_Indicator) "Emissive" (* (Variables|Default|GetEmissive%20Intensity) (select (Variables|Default|GetOFF=Color2) true (Variables|Default|GetON))))
  (Rendering|Material|SetVectorParameterValueonMaterials (Variables|Default|GetSM_Indicator) "Color" (Math|Conversions|ToVector(LinearColor) (Math|Conversions|ToLinearColor(Color) (select (Variables|Default|GetOFF=Color2) (select (Variables|Default|GetON) _indicator_color (Variables|Default|GetIndicator%20Color%20When%20OFF)) _indicator_color)))))