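; BP_EnemyGuardsDrone is a guard drone enemy Blueprint that handles the drone's fall when it dies.
; On BeginPlay it binds a custom event to the OnDeath delegate of its health component.
; That event disables actor collision and plays the DroneFallingDeath timeline, which adds its track value as a vertical world offset on each update, without sweeping.
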(event Custom|CustomEvent
  (Collision|SetActorEnableCollision false)
  (bind _falltrack_0 (Timeline|DroneFallingDeath Play)
    (:Update
      (Transformation|AddActorWorldOffset (Math|Vector|MakeVector 0.0 0.0 _falltrack_0)))))

(event EventBeginPlay
  (EventDispatchers|BindEventtoOnDeath (Variables|Default|GetAC_HealthComp) (delegate Custom|CustomEvent)))

(event Collision|EventActorBeginOverlap
  (params (OtherActor :type Actor%20Object%20Reference))
  (|CallParentFunction OtherActor) ; This node is disabled and will not be called.\nDrag off pins to build functionality.
)

(event EventTick
  (params (DeltaSeconds :type Float%20%28single-precision%29))
  (|CallParentFunction DeltaSeconds) ; This node is disabled and will not be called.\nDrag off pins to build functionality.
)

(fn ConstructionScript
  (|CallParentFunction))