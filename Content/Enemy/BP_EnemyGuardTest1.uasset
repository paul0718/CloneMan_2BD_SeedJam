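; Test enemy guard that turns toward the player character and fires projectiles at it when seen.
; Pawn sensing stores the top-down character as target, then a visibility trace with persistent debug lines confirms line of sight.
; A hit spawns a projectile and calls ApplyDamage with no inputs, using a CanAttack flag with a delayed reset.
; Tick smoothly rotates toward the target but also re-enables CanAttack every frame, bypassing that cooldown.
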(event OnSeePawn(PawnSensing)
  (params (Pawn :type Pawn%20Object%20Reference))
  (bind _asbp_top_down_character (Utilities|Casting|CastToBP_TopDownCharacter Pawn))
  (bind _output_get (Variables|Default|SetTargetActor _asbp_top_down_character))
  (bind _outhit (Collision|LineTraceByChannel (Transformation|GetActorLocation) (Transformation|GetActorLocation (Variables|Default|GetTargetActor)) "TraceTypeQuery1" false 0 "Persistent"))
  (if (== _output_get (.HitActor (Collision|BreakHitResult _outhit)))
    (if (Variables|Default|GetCanAttack)
      (Game|SpawnActorfromClass "/Game/TopDown/Blueprints/BP_Projectile.BP_Projectile_C" (Transformation|GetWorldTransform (Variables|Default|GetProjectileSpawn)) "Undefined" "MultiplyWithRoot" 0 0)
      (Game|Damage|ApplyDamage 0 0.0 0 0)
      (Variables|Default|SetCanAttack false)
      (Utilities|FlowControl|Delay 0.3)
      (Variables|Default|SetCanAttack true))))

(event EventBeginPlay)

(event Collision|EventActorBeginOverlap
  (params (OtherActor :type Actor%20Object%20Reference)))

(event EventTick
  (params (DeltaSeconds :type Float%20%28single-precision%29))
  (if (Utilities|IsValid (Variables|Default|GetTargetActor))
    (Transformation|SetActorRotation (Math|Interpolation|RInterpTo (Transformation|GetActorRotation) (Math|Rotator|FindRelativeLookatRotation (Math|Conversions|ToTransform(Vector) (Transformation|GetActorLocation)) (Transformation|GetActorLocation (Variables|Default|GetTargetActor))) DeltaSeconds 2.0))
    (Variables|Default|SetCanAttack true)))

(fn ConstructionScript)