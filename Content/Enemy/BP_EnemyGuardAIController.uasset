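; AI controller for enemy guards that runs the guard behavior tree and tracks the player through AI perception.
; Sensing a Cloneman-controlled top-down character updates the canSeePlayer and TargetActor blackboard keys; losing sight clears the target and prints a debug trace of the blocker.
; Death bindings reset the keys when the player dies, and on guard death stop the tree, unpossess, loosen capsule collision, and play a death animation and sound.
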(event OnTargetPerceptionUpdated(AIPerception)
  (params (Actor :type Actor%20Object%20Reference) (Stimulus :type AI%20Stimulus%20Structure))
  (bind _bsuccessfullysensed (Utilities|Struct|BreakAIStimulus Stimulus))
  (bind _blackboard (Variables|Default|GetBlackboard))
  (bind _asbp_top_down_character (Utilities|Casting|CastToBP_TopDownCharacter Actor))
  (bind _asbp_cloneman_controller (Utilities|Casting|CastToBP_ClonemanController (Pawn|GetController _asbp_top_down_character)))
  (if (Utilities|IsValid _asbp_cloneman_controller)
    (bind _output_get (Variables|Default|SetPlayerActor _asbp_top_down_character))
    (EventDispatchers|BindEventtoOnDeath (Variables|/Game/TopDown/Blueprints/BP_TopDownCharacter.BP_TopDownCharacter_C|GetAC_HealthComp _output_get) (delegate Custom|onPlayerDeath))
    (AI|Components|Blackboard|SetValueasBool _blackboard (Utilities|Name|MakeLiteralName "canSeePlayer") _bsuccessfullysensed)
    (if _bsuccessfullysensed
      (AI|Components|Blackboard|SetValueasObject _blackboard (Utilities|Name|MakeLiteralName "TargetActor") (Variables|Default|GetPlayerActor))
      (else
        (bind _outhit (Collision|LineTraceByChannel (Transformation|GetActorLocation (Variables|Default|GetEnemyActor)) (Transformation|GetActorLocation (Variables|Default|GetPlayerActor)) "TraceTypeQuery1" false 0 "None"))
        (Development|PrintString "Blocked by:")
        (Development|PrintString (Utilities|GetDisplayName (.HitActor (Collision|BreakHitResult _outhit))))
        (AI|Components|Blackboard|ClearValue _blackboard (Utilities|Name|MakeLiteralName "TargetActor"))))))

(event Custom|onSelfDeath
  (bind _enemyactor (Variables|Default|GetEnemyActor))
  (bind _enemyactor_2 (Variables|Default|GetEnemyActor))
  (bind _capsulecomponent (Variables|/Script/Engine.Character|GetCapsuleComponent _enemyactor))
  (bind _mesh (Variables|/Script/Engine.Character|GetMesh _enemyactor_2))
  (Variables|Default|SetisDead true)
  (AI|Logic|StopLogic (Variables|Default|GetBrainComponent) "")
  (Pawn|UnPossess)
  (Development|PrintString "Enemy dead animation")
  (Collision|SetCollisionResponsetoChannel _capsulecomponent "ECC_Pawn" "ECR_Ignore")
  (Collision|SetCollisionResponsetoChannel _capsulecomponent "ECC_WorldDynamic" "ECR_Ignore")
  (Components|Animation|SetAnimationMode _mesh "AnimationSingleNode" true)
  (Components|Animation|PlayAnimation _mesh "/Game/Animation/FallingBackDeath_UE.FallingBackDeath_UE" false)
  (Utilities|FlowControl|Delay 0.5)
  (Audio|PlaySoundatLocation "/Game/SoundEffectsPlaceHolders/NonPlaceHolders/SFX_GP_Enemy_Death.SFX_GP_Enemy_Death" (Transformation|GetActorLocation _enemyactor_2) "0, 0, 0" 1.0 1.0 0.0 "/Game/SoundEffectsPlaceHolders/BasicSoundAttenuation.BasicSoundAttenuation" 0 0 0))

(event Custom|onPlayerDeath
  (bind _blackboard (Variables|Default|GetBlackboard))
  (AI|Components|Blackboard|SetValueasBool _blackboard (Utilities|Name|MakeLiteralName "canSeePlayer") false)
  (AI|Components|Blackboard|ClearValue _blackboard (Utilities|Name|MakeLiteralName "TargetActor")))

(event EventBeginPlay
  (AI|RunBehaviorTree "/Game/Enemy/BT_EnemyGuardAI.BT_EnemyGuardAI"))

(event EventTick
  (params (DeltaSeconds :type Float%20%28single-precision%29)))

(event EventPossess
  (params (PossessedPawn :type Pawn%20Object%20Reference))
  (bind _asbp_enemy_guards (Utilities|Casting|CastToBP_EnemyGuards PossessedPawn))
  (bind _output_get (Variables|Default|SetEnemyActor _asbp_enemy_guards))
  (if (not (Variables|Default|GetisDead))
    (EventDispatchers|BindEventtoOnDeath (Variables|/Game/Enemy/BP_EnemyGuards.BP_EnemyGuards_C|GetAC_HealthComp _output_get) (delegate Custom|onSelfDeath))))

(fn ConstructionScript)