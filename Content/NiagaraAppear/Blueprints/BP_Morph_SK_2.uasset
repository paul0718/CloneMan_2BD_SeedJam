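; Actor that loops a Niagara morph effect between two skeletal meshes.
; On BeginPlay it attaches NS_Morph_SK_F_2, passes it color, spawn rate and both meshes, and swaps in morph materials.
; Two timelines, the second delayed, drive Amount and Amount1 in MPC_Morph_SK_1, then the system is destroyed and the cycle restarts.
; Initial amounts and emissive color are written to a different collection, MPC_Morph_SK.
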(event EventBeginPlay
  (bind _emissive_color (Variables|Default|GetEmissive%20Color))
  (bind _skeletal_mesh_component_0 (Variables|Default|GetSkeletal%20Mesh%20Component_0))
  (bind _skeletal_mesh_component_1 (Variables|Default|GetSkeletal%20Mesh%20Component_1))
  (bind _skeletalmeshcomponent (Variables|/Script/Engine.SkeletalMeshActor|GetSkeletalMeshComponent _skeletal_mesh_component_0))
  (bind _skeletalmeshcomponent_2 (Variables|/Script/Engine.SkeletalMeshActor|GetSkeletalMeshComponent _skeletal_mesh_component_1))
  (bind _returnvalue (Niagara|SpawnSystemAttached "/Game/NiagaraAppear/Niagara/NS_Morph_SK_F_2.NS_Morph_SK_F_2" (Variables|Default|GetDefaultSceneRoot) "None" "0, 0, 0" "0, 0, 0" "KeepRelativeOffset" false :!label _label))
  (CallFunction|NiagaraSetting _returnvalue _emissive_color (Variables|Default|GetSpawn%20Rate))
  (Class|NiagaraFunctionLibrary|OverrideSystemUserVariableSkeletalMeshComponent _returnvalue "Skeletal Mesh0" _skeletalmeshcomponent)
  (Rendering|Material|SetMaterial _skeletalmeshcomponent 0 (Variables|Default|GetM_Mesh_1))
  (Rendering|Material|SetMaterial _skeletalmeshcomponent 1 (Variables|Default|GetM_Mesh_2))
  (Class|NiagaraFunctionLibrary|OverrideSystemUserVariableSkeletalMeshComponent _returnvalue "Skeletal Mesh1" _skeletalmeshcomponent_2)
  (Rendering|Material|SetMaterial _skeletalmeshcomponent_2 0 (Variables|Default|GetM_Mesh_3))
  (Rendering|Material|SetMaterial _skeletalmeshcomponent_2 1 (Variables|Default|GetM_Mesh_4))
  (Rendering|Material|SetScalarParameterValue "/Game/NiagaraAppear/DemoRoom/SkeletalMeshExample/Character/Materials/Morph/MPC_Morph_SK.MPC_Morph_SK" "Amount" 1.0 :!class /Script/Engine.KismetMaterialLibrary)
  (Rendering|Material|SetScalarParameterValue "/Game/NiagaraAppear/DemoRoom/SkeletalMeshExample/Character/Materials/Morph/MPC_Morph_SK.MPC_Morph_SK" "Amount1" 0.0 :!class /Script/Engine.KismetMaterialLibrary)
  (Utilities|FlowControl|Sequence
    (:then_0
      (bind _newtrack_0 (Timeline|Timeline_0 PlayFromStart)
        (:Update
          (Rendering|Material|SetScalarParameterValue "/Game/NiagaraAppear/DemoRoom/SkeletalMeshExample/Character/Materials/Morph/MPC_Morph_SK_1.MPC_Morph_SK_1" "Amount" _newtrack_0 :!class /Script/Engine.KismetMaterialLibrary))))
    (:then_1
      (Utilities|FlowControl|Delay 4.0)
      (bind _newtrack_0_2 (Timeline|Timeline_1 PlayFromStart)
        (:Update
          (Rendering|Material|SetScalarParameterValue "/Game/NiagaraAppear/DemoRoom/SkeletalMeshExample/Character/Materials/Morph/MPC_Morph_SK_1.MPC_Morph_SK_1" "Amount1" _newtrack_0_2 :!class /Script/Engine.KismetMaterialLibrary))
        (:Finished
          (Utilities|FlowControl|Delay 2.0)
          (Components|DestroyComponent _returnvalue)
          (Rendering|Material|SetScalarParameterValue "/Game/NiagaraAppear/DemoRoom/SkeletalMeshExample/Character/Materials/Morph/MPC_Morph_SK_1.MPC_Morph_SK_1" "Amount" 1.0 :!class /Script/Engine.KismetMaterialLibrary)
          (Rendering|Material|SetScalarParameterValue "/Game/NiagaraAppear/DemoRoom/SkeletalMeshExample/Character/Materials/Morph/MPC_Morph_SK_1.MPC_Morph_SK_1" "Amount1" 0.0 :!class /Script/Engine.KismetMaterialLibrary)
          (goto _label))))
    (:then_2
      (Rendering|Material|SetVectorParameterValue "/Game/NiagaraAppear/DemoRoom/SkeletalMeshExample/Character/Materials/Morph/MPC_Morph_SK.MPC_Morph_SK" "Emissive" _emissive_color :!class /Script/Engine.KismetMaterialLibrary))))

(fn ConstructionScript)

(fn NiagaraSetting
  (params (Target :type Niagara%20Component%20Object%20Reference) (Emissive%20Color :type Linear%20Color%20Structure%20%28by%20ref%29) (SpawnRate :type Float%20%28double-precision%29))
  (Niagara|SetNiagaraVariable(LinearColor) Target "Emissive Color" Emissive%20Color)
  (Niagara|SetNiagaraVariable(Float) Target "SpawnRate" SpawnRate))